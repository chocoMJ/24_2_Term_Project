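; Player inventory component that stores items in main slots plus button slots, and toggles the inventory and work menu widgets on Tab and R.
; E sphere-traces near the player's feet for a BP_Item, stacking it up to a cap or filling an empty slot.
; Widget drop events move, swap, merge or trash items, then reload the UI.
; Button slots share the index range after main slots and filter swaps by allowed item names.
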(event Custom|MouseDropButton
  (params (TargetIndex :type Integer) (BeforeInventorySystem :type WB%20Inventory%20Object%20Reference) (BeforeIndex :type Integer))
  (CallFunction|ChangeSlotButton TargetIndex BeforeInventorySystem BeforeIndex))

(event Custom|MouseDrop
  (params (TargetIndex :type Integer) (BeforeInventorySystem :type WB%20Inventory%20Object%20Reference) (BeforeIndex :type Integer))
  (CallFunction|ChangeSlot TargetIndex BeforeInventorySystem BeforeIndex))

(event Custom|Trash
  (params (BeforeInventorySystem :type WB%20Inventory%20Object%20Reference) (Before%20Index :type Integer))
  (CallFunction|TrashItem BeforeInventorySystem Before%20Index))

(event EventBeginPlay
  (bind _self self)
  (bind _returnvalue (UserInterface|CreateWidget "/Game/Inventory_UI/WB_Inventory.WB_Inventory_C"))
  (Variables|Default|SetWB_Inventory _returnvalue)
  (Utilities|Array|Resize (Variables|Default|Getslots) 35)
  (Utilities|Array|Resize (Variables|Default|Getslots_button) 6)
  (Default|LoadInventory (Variables|Default|GetWB_Inventory) _self)
  (Default|LoadInventoryButton (Variables|Default|GetWB_Inventory) _self)
  (bind _returnvalue_2 (UserInterface|CreateWidget "/Game/WorkMenu_UI/WB_WorkMenu.WB_WorkMenu_C" 0 _self (Variables|Default|GetWB_Inventory)))
  (Variables|Default|SetWB_WorkMenu _returnvalue_2)
  (Default|LoadTrashcan (Variables|Default|GetWB_Inventory) _self))

(event Input|KeyboardEvents|Tab
  (params (Key :type Key%20Structure :default "None"))
  (bind _returnvalue (Game|GetPlayerController 0))
  (bind _returnvalue_2 (Game|GetPlayerController 0))
  (bind _wb_inventory (Variables|Default|GetWB_Inventory))
  (:Pressed
    (if (Widget|IsVisible (Variables|Default|GetWB_Inventory))
      (Widget|RemovefromParent _wb_inventory)
      (Variables|/Script/Engine.PlayerController|SetbShowMouseCursor _returnvalue_2 false)
      (Input|SetInputModeGameOnly _returnvalue_2 false)
      (else
        (Variables|/Script/Engine.PlayerController|SetbShowMouseCursor _returnvalue true)
        (Input|SetInputModeGameandUI _returnvalue 0 "DoNotLock" true false)
        (UserInterface|Viewport|AddtoViewport _wb_inventory 0)))))

(event Input|KeyboardEvents|R
  (params (Key :type Key%20Structure :default "None"))
  (bind _returnvalue (Game|GetPlayerController 0))
  (bind _returnvalue_2 (Game|GetPlayerController 0))
  (bind _wb_workmenu (Variables|Default|GetWB_WorkMenu))
  (:Pressed
    (if (Widget|IsVisible (Variables|Default|GetWB_WorkMenu))
      (Widget|RemovefromParent _wb_workmenu)
      (Variables|/Script/Engine.PlayerController|SetbShowMouseCursor _returnvalue false)
      (Input|SetInputModeGameOnly _returnvalue false)
      (else
        (Variables|/Script/Engine.PlayerController|SetbShowMouseCursor _returnvalue_2 true)
        (Input|SetInputModeGameandUI _returnvalue_2 0 "DoNotLock" true false)
        (UserInterface|Viewport|AddtoViewport _wb_workmenu 0)))))

(event Input|KeyboardEvents|E
  (params (Key :type Key%20Structure :default "None"))
  (bind _returnvalue (Game|GetPlayerCharacter 0))
  (bind _returnvalue_2 (Transformation|GetActorLocation _returnvalue))
  (bind _returnvalue_3 (- _returnvalue_2 "0.000000,0.000000,65.000000"))
  (:Pressed
    (bind _outhit (Collision|SphereTraceByChannel _returnvalue_3 _returnvalue_3 1.2e+02 "TraceTypeQuery1" false 0 "None"))
    (bind _asbp_item (Utilities|Casting|CastToBP_Item (.HitActor (Collision|BreakHitResult _outhit))))
    (for (_array_element _array_index) (Variables|Default|Getslots)
      (Utilities|IsValid _asbp_item
        (:Is%20Valid
          (if (Math|Boolean|ANDBoolean (Utilities|Enum|Equal(Enum) (Utilities|Text|ToText(Name) (.Name (Utilities|Struct|BreakS_ItemStructure _array_element))) (Utilities|Text|ToText(Name) (.Name (Utilities|Struct|BreakS_ItemStructure (Variables|/Game/Inventory_UI/BP_Item.BP_Item_C|GetItem _asbp_item))))) (.Stackable (Utilities|Struct|BreakS_ItemStructure (Variables|/Game/Inventory_UI/BP_Item.BP_Item_C|GetItem _asbp_item))) (<= (+ (.Quantity (Utilities|Struct|BreakS_ItemStructure _array_element)) (.Quantity (Utilities|Struct|BreakS_ItemStructure (Variables|/Game/Inventory_UI/BP_Item.BP_Item_C|GetItem _asbp_item)))) 10))
            (Utilities|Array|SetArrayElem (Variables|Default|Getslots) _array_index (Utilities|Struct|MakeS_ItemStructure (.name (Variables|/Game/Inventory_UI/BP_Item.BP_Item_C|GetItem _asbp_item)) (.stackable (Variables|/Game/Inventory_UI/BP_Item.BP_Item_C|GetItem _asbp_item)) (+ (.Quantity (Utilities|Struct|BreakS_ItemStructure _array_element)) (.Quantity (Utilities|Struct|BreakS_ItemStructure (Variables|/Game/Inventory_UI/BP_Item.BP_Item_C|GetItem _asbp_item)))) (.thumnail (Variables|/Game/Inventory_UI/BP_Item.BP_Item_C|GetItem _asbp_item)) (.mesh (Variables|/Game/Inventory_UI/BP_Item.BP_Item_C|GetItem _asbp_item))))
            (Default|LoadInventory (Variables|Default|GetWB_Inventory) self :!label _label)
            (Actor|DestroyActor _asbp_item)
            (elif (== (.Quantity (Utilities|Struct|BreakS_ItemStructure _array_element)) 0)
              (Utilities|Array|SetArrayElem (Variables|Default|Getslots) _array_index (Variables|/Game/Inventory_UI/BP_Item.BP_Item_C|GetItem _asbp_item))
              (goto _label))))))))

(fn ChangeSlot
  (params (TargetIndex :type Integer) (BeforeInventorySystem :type WB%20Inventory%20Object%20Reference) (BeforeIndex :type Integer))
  (bind _slots (Variables|Default|Getslots))
  (bind _slots_2 (Variables|Default|Getslots))
  (bind _slots_3 (Variables|Default|Getslots))
  (bind _slots_4 (Variables|Default|Getslots))
  (bind _output (Utilities|Array|Get(acopy) _slots TargetIndex))
  (bind _output_2 (Utilities|Array|Get(acopy) _slots_3 TargetIndex))
  (bind _output_3 (Utilities|Array|Get(acopy) _slots_2 TargetIndex))
  (bind _output_4 (Utilities|Array|Get(acopy) _slots_4 BeforeIndex))
  (bind _quantity (Utilities|Struct|BreakS_ItemStructure _output_4))
  (bind (_name _stackable) (Utilities|Struct|BreakS_ItemStructure _output_2))
  (bind (_name_2 _stackable_2) (Utilities|Struct|BreakS_ItemStructure _output))
  (bind _quantity_2 (Utilities|Struct|BreakS_ItemStructure _output_3))
  (bind _returnvalue (+ _quantity_2 _quantity))
  (if (<= BeforeIndex 34)
    (LocalVariables|SetLocalSlot (Utilities|Array|Get(acopy) (Variables|Default|Getslots) BeforeIndex))
    (if (>= TargetIndex 0)
      (if (!= (.Name (Utilities|Struct|BreakS_ItemStructure (LocalVariables|GetLocalSlot))) _name_2)
        (Utilities|Array|SetArrayElem (Variables|Default|Getslots) BeforeIndex (Utilities|Array|Get(acopy) (Variables|Default|Getslots) TargetIndex) :!label _label)
        (Utilities|Array|SetArrayElem (Variables|Default|Getslots) TargetIndex (LocalVariables|GetLocalSlot))
        (Default|LoadInventory BeforeInventorySystem self)
        (elif (and (.Stackable (Utilities|Struct|BreakS_ItemStructure (LocalVariables|GetLocalSlot))) _stackable_2)
          (if (<= _returnvalue 10)
            (Utilities|Array|SetArrayElem :TargetArray (Variables|Default|Getslots) :Index BeforeIndex)
            (Utilities|Array|SetArrayElem (Variables|Default|Getslots) TargetIndex (Utilities|Struct|MakeS_ItemStructure (.Name (Utilities|Struct|BreakS_ItemStructure (LocalVariables|GetLocalSlot))) (.Stackable (Utilities|Struct|BreakS_ItemStructure (LocalVariables|GetLocalSlot))) (+ (.Quantity (Utilities|Struct|BreakS_ItemStructure (LocalVariables|GetLocalSlot))) _quantity_2) (.Thumnail (Utilities|Struct|BreakS_ItemStructure (LocalVariables|GetLocalSlot))) (.Mesh (Utilities|Struct|BreakS_ItemStructure (LocalVariables|GetLocalSlot)))))
            (Default|LoadInventory BeforeInventorySystem self)
            (else
              (Utilities|Array|SetArrayElem (Variables|Default|Getslots) BeforeIndex (Utilities|Struct|MakeS_ItemStructure (.Name (Utilities|Struct|BreakS_ItemStructure (LocalVariables|GetLocalSlot))) (.Stackable (Utilities|Struct|BreakS_ItemStructure (LocalVariables|GetLocalSlot))) (- _returnvalue 10) (.Thumnail (Utilities|Struct|BreakS_ItemStructure (LocalVariables|GetLocalSlot))) (.Mesh (Utilities|Struct|BreakS_ItemStructure (LocalVariables|GetLocalSlot)))))
              (Utilities|Array|SetArrayElem (Variables|Default|Getslots) TargetIndex (Utilities|Struct|MakeS_ItemStructure (.Name (Utilities|Struct|BreakS_ItemStructure (LocalVariables|GetLocalSlot))) (.Stackable (Utilities|Struct|BreakS_ItemStructure (LocalVariables|GetLocalSlot))) 10 (.Thumnail (Utilities|Struct|BreakS_ItemStructure (LocalVariables|GetLocalSlot))) (.Mesh (Utilities|Struct|BreakS_ItemStructure (LocalVariables|GetLocalSlot)))))
              (Default|LoadInventory BeforeInventorySystem self)))
          (else
            (goto _label)))))
    (elif true
      (LocalVariables|SetLocalSlot (Variables|/Game/Inventory_UI/WB_Slot_Button.WB_Slot_Button_C|GetItem (Utilities|Array|Get(acopy) (Variables|Default|Getslots_button) (- BeforeIndex 35))))
      (if (>= TargetIndex 0)
        (if (!= (.Name (Utilities|Struct|BreakS_ItemStructure (LocalVariables|GetLocalSlot))) _name)
          (if (== _name "")
            (Utilities|Array|SetArrayElem (Variables|Default|Getslots) TargetIndex (LocalVariables|GetLocalSlot))
            (Variables|Default|SetSlotItem (Utilities|Array|Get(acopy) (Variables|Default|Getslots_button) (- BeforeIndex 35)))
            (Variables|/Game/Inventory_UI/WB_Slot_Button.WB_Slot_Button_C|SetItem (Variables|Default|GetSlotItem) "")
            (Utilities|Array|SetArrayElem (Variables|Default|Getslots_button) (- BeforeIndex 35) (Variables|Default|GetSlotItem))
            (Default|LoadInventoryButton BeforeInventorySystem self)
            (Default|LoadInventory BeforeInventorySystem self))
          (elif (and (.Stackable (Utilities|Struct|BreakS_ItemStructure (LocalVariables|GetLocalSlot))) _stackable)
            (if (<= (+ (Utilities|Struct|BreakS_ItemStructure (Variables|/Game/Inventory_UI/WB_Slot_Button.WB_Slot_Button_C|GetItem (Utilities|Array|Get(acopy) (Variables|Default|Getslots_button) (- BeforeIndex 35)))) (Utilities|Struct|BreakS_ItemStructure (LocalVariables|GetLocalSlot))) 10)
              (Utilities|Array|SetArrayElem (Variables|Default|Getslots) TargetIndex (Utilities|Struct|MakeS_ItemStructure (.Name (Utilities|Struct|BreakS_ItemStructure (LocalVariables|GetLocalSlot))) (.Stackable (Utilities|Struct|BreakS_ItemStructure (LocalVariables|GetLocalSlot))) (+ (.Quantity (Utilities|Struct|BreakS_ItemStructure (LocalVariables|GetLocalSlot))) (Utilities|Struct|BreakS_ItemStructure (Variables|/Game/Inventory_UI/WB_Slot_Button.WB_Slot_Button_C|GetItem (Utilities|Array|Get(acopy) (Variables|Default|Getslots_button) (- BeforeIndex 35))))) (.Thumnail (Utilities|Struct|BreakS_ItemStructure (LocalVariables|GetLocalSlot))) (.Mesh (Utilities|Struct|BreakS_ItemStructure (LocalVariables|GetLocalSlot)))))
              (Variables|Default|SetSlotItem (Utilities|Array|Get(acopy) (Variables|Default|Getslots_button) (- BeforeIndex 35)))
              (Variables|/Game/Inventory_UI/WB_Slot_Button.WB_Slot_Button_C|SetItem (Variables|Default|GetSlotItem) "")
              (Utilities|Array|SetArrayElem (Variables|Default|Getslots_button) (- BeforeIndex 35) (Variables|Default|GetSlotItem))
              (Default|LoadInventoryButton BeforeInventorySystem self)
              (Default|LoadInventory BeforeInventorySystem self)
              (else
                (Variables|Default|SetSlotItem (Utilities|Array|Get(acopy) (Variables|Default|Getslots_button) (- BeforeIndex 35)))
                (Variables|/Game/Inventory_UI/WB_Slot_Button.WB_Slot_Button_C|SetItem (Variables|Default|GetSlotItem) (Utilities|Struct|MakeS_ItemStructure (.Name (Utilities|Struct|BreakS_ItemStructure (LocalVariables|GetLocalSlot))) (.Stackable (Utilities|Struct|BreakS_ItemStructure (LocalVariables|GetLocalSlot))) (- (+ (Utilities|Struct|BreakS_ItemStructure (Variables|/Game/Inventory_UI/WB_Slot_Button.WB_Slot_Button_C|GetItem (Utilities|Array|Get(acopy) (Variables|Default|Getslots_button) (- BeforeIndex 35)))) (Utilities|Struct|BreakS_ItemStructure (LocalVariables|GetLocalSlot))) 10) (.Thumnail (Utilities|Struct|BreakS_ItemStructure (LocalVariables|GetLocalSlot))) (.Mesh (Utilities|Struct|BreakS_ItemStructure (LocalVariables|GetLocalSlot)))))
                (Utilities|Array|SetArrayElem (Variables|Default|Getslots_button) (- BeforeIndex 35) (Variables|Default|GetSlotItem))
                (Utilities|Array|SetArrayElem (Variables|Default|Getslots) TargetIndex (Utilities|Struct|MakeS_ItemStructure (.Name (Utilities|Struct|BreakS_ItemStructure (LocalVariables|GetLocalSlot))) (.Stackable (Utilities|Struct|BreakS_ItemStructure (LocalVariables|GetLocalSlot))) 10 (.Thumnail (Utilities|Struct|BreakS_ItemStructure (LocalVariables|GetLocalSlot))) (.Mesh (Utilities|Struct|BreakS_ItemStructure (LocalVariables|GetLocalSlot)))))
                (Default|LoadInventoryButton BeforeInventorySystem self)
                (Default|LoadInventory BeforeInventorySystem self)))))))))

(fn ChangeSlotButton
  (params (TargetIndex :type Integer) (BeforeInventorySystem :type WB%20Inventory%20Object%20Reference) (BeforeIndex :type Integer))
  (if (< BeforeIndex 35)
    (if true
      (LocalVariables|SetLocal%20Slot (Utilities|Array|Get(acopy) (Variables|Default|Getslots) BeforeIndex))
      (if (>= TargetIndex 0)
        (if (!= (.Name (Utilities|Struct|BreakS_ItemStructure (LocalVariables|GetLocal%20Slot))) (.Name (Utilities|Struct|BreakS_ItemStructure (Variables|/Game/Inventory_UI/WB_Slot_Button.WB_Slot_Button_C|GetItem (Utilities|Array|Get(acopy) (Variables|Default|Getslots_button) (- TargetIndex 35))))))
          (bind _array_element (Utilities|Array|ForEachLoopwithBreak (Variables|/Game/Inventory_UI/WB_Slot_Button.WB_Slot_Button_C|Getitemname (Utilities|Array|Get(acopy) (Variables|Default|Getslots_button) (- TargetIndex 35))))
            (:LoopBody
              (if (== _array_element (.Name (Utilities|Struct|BreakS_ItemStructure (LocalVariables|GetLocal%20Slot))))
                (Utilities|Array|SetArrayElem (Variables|Default|Getslots) BeforeIndex (Variables|/Game/Inventory_UI/WB_Slot_Button.WB_Slot_Button_C|GetItem (Utilities|Array|Get(acopy) (Variables|Default|Getslots_button) (- TargetIndex 35))))
                (Variables|Default|SetSlotItem (Utilities|Array|Get(acopy) (Variables|Default|Getslots_button) (- TargetIndex 35)))
                (Variables|/Game/Inventory_UI/WB_Slot_Button.WB_Slot_Button_C|SetItem (Variables|Default|GetSlotItem) (LocalVariables|GetLocal%20Slot))
                (Utilities|Array|SetArrayElem (Variables|Default|Getslots_button) (- TargetIndex 35) (Variables|Default|GetSlotItem))
                (Default|LoadInventoryButton BeforeInventorySystem self)
                (Default|LoadInventory BeforeInventorySystem self))))
          (elif (and (.Stackable (Utilities|Struct|BreakS_ItemStructure (LocalVariables|GetLocal%20Slot))) (.Stackable (Utilities|Struct|BreakS_ItemStructure (Variables|/Game/Inventory_UI/WB_Slot_Button.WB_Slot_Button_C|GetItem (Utilities|Array|Get(acopy) (Variables|Default|Getslots_button) (- TargetIndex 35))))))
            (if (<= (+ (Utilities|Struct|BreakS_ItemStructure (Variables|/Game/Inventory_UI/WB_Slot_Button.WB_Slot_Button_C|GetItem (Utilities|Array|Get(acopy) (Variables|Default|Getslots_button) (- TargetIndex 35)))) (Utilities|Struct|BreakS_ItemStructure (LocalVariables|GetLocal%20Slot))) 10)
              (Utilities|Array|SetArrayElem :TargetArray (Variables|Default|Getslots) :Index BeforeIndex)
              (Variables|Default|SetSlotItem (Utilities|Array|Get(acopy) (Variables|Default|Getslots_button) (- TargetIndex 35)))
              (Variables|/Game/Inventory_UI/WB_Slot_Button.WB_Slot_Button_C|SetItem (Variables|Default|GetSlotItem) (Utilities|Struct|MakeS_ItemStructure (.Name (Utilities|Struct|BreakS_ItemStructure (LocalVariables|GetLocal%20Slot))) (.Stackable (Utilities|Struct|BreakS_ItemStructure (LocalVariables|GetLocal%20Slot))) (+ (.Quantity (Utilities|Struct|BreakS_ItemStructure (LocalVariables|GetLocal%20Slot))) (Utilities|Struct|BreakS_ItemStructure (Variables|/Game/Inventory_UI/WB_Slot_Button.WB_Slot_Button_C|GetItem (Utilities|Array|Get(acopy) (Variables|Default|Getslots_button) (- TargetIndex 35))))) (.Thumnail (Utilities|Struct|BreakS_ItemStructure (LocalVariables|GetLocal%20Slot))) (.Mesh (Utilities|Struct|BreakS_ItemStructure (LocalVariables|GetLocal%20Slot)))))
              (Utilities|Array|SetArrayElem (Variables|Default|Getslots_button) (- TargetIndex 35) (Variables|Default|GetSlotItem))
              (Default|LoadInventoryButton BeforeInventorySystem self)
              (Default|LoadInventory BeforeInventorySystem self)
              (else
                (Utilities|Array|SetArrayElem (Variables|Default|Getslots) BeforeIndex (Utilities|Struct|MakeS_ItemStructure (.Name (Utilities|Struct|BreakS_ItemStructure (LocalVariables|GetLocal%20Slot))) (.Stackable (Utilities|Struct|BreakS_ItemStructure (LocalVariables|GetLocal%20Slot))) (- (+ (Utilities|Struct|BreakS_ItemStructure (Variables|/Game/Inventory_UI/WB_Slot_Button.WB_Slot_Button_C|GetItem (Utilities|Array|Get(acopy) (Variables|Default|Getslots_button) (- TargetIndex 35)))) (Utilities|Struct|BreakS_ItemStructure (LocalVariables|GetLocal%20Slot))) 10) (.Thumnail (Utilities|Struct|BreakS_ItemStructure (LocalVariables|GetLocal%20Slot))) (.Mesh (Utilities|Struct|BreakS_ItemStructure (LocalVariables|GetLocal%20Slot)))))
                (Variables|Default|SetSlotItem (Utilities|Array|Get(acopy) (Variables|Default|Getslots_button) (- TargetIndex 35)))
                (Variables|/Game/Inventory_UI/WB_Slot_Button.WB_Slot_Button_C|SetItem (Variables|Default|GetSlotItem) (Utilities|Struct|MakeS_ItemStructure (.Name (Utilities|Struct|BreakS_ItemStructure (LocalVariables|GetLocal%20Slot))) (.Stackable (Utilities|Struct|BreakS_ItemStructure (LocalVariables|GetLocal%20Slot))) 10 (.Thumnail (Utilities|Struct|BreakS_ItemStructure (LocalVariables|GetLocal%20Slot))) (.Mesh (Utilities|Struct|BreakS_ItemStructure (LocalVariables|GetLocal%20Slot)))))
                (Utilities|Array|SetArrayElem (Variables|Default|Getslots_button) (- TargetIndex 35) (Variables|Default|GetSlotItem))
                (Default|LoadInventoryButton BeforeInventorySystem self)
                (Default|LoadInventory BeforeInventorySystem self)))))))))

(fn TrashItem
  (params (BeforeInventorySystem :type WB%20Inventory%20Object%20Reference) (Before%20Index :type Integer))
  (Utilities|Array|SetArrayElem :TargetArray (Variables|Default|Getslots) :Index Before%20Index)
  (Default|LoadInventory BeforeInventorySystem self))