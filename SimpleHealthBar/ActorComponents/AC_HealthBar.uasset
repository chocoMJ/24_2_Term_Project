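; Actor component that manages an owner's health, shield, mana, level and status conditions, and creates its health bar widget.
; Shield absorbs damage before health, while level-ups scale maximum health and mana from Settings, with optional full heal.
; Poison and Burn spawn as condition actors attached to the owner, and change dispatchers broadcast updates.
; The bar is a screen-space widget component added at runtime, alongside debug printouts, widget and test keys.
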(event Custom|OnLevelChange_Event
  (if (> (Variables|Don'tEdit|GetLevel) 1)
    (CallFunction|SetHealthandManaonLevelUp)))

(event EventBeginPlay
  (if (Variables|!HealthBarSettings|GetDebug)
    (Utilities|AddDebugWidget))
  (CallFunction|SetStartingLevel)
  (CallFunction|SetBaseHealthandManaValues)
  (EventDispatchers|BindEventtoOnLevelChange (delegate Custom|OnLevelChange_Event))
  (Utilities|AddWidget)
  (Default|CallOnLevelChange))

(event EventTick
  (params (DeltaSeconds :type Float%20%28single-precision%29))
  ;[1 0.4074 0] DEBUG
  (if (Variables|!HealthBarSettings|GetDebug)
    (Development|PrintString (Utilities|String|Append (Utilities|String|Append "HP: " (Utilities|String|ToString(Integer) (Variables|Don'tEdit|GetCurrentHealth)) " / " (Utilities|String|ToString(Integer) (Variables|Don'tEdit|GetMaxHealth)) " 
") (Utilities|String|Append "MANA: " (Utilities|String|ToString(Integer) (Variables|Don'tEdit|GetCurrentMana)) " / " (Utilities|String|ToString(Integer) (Variables|Don'tEdit|GetMaxMana)) " 
")) true true "(R=0.000000,G=1.000000,B=0.102367,A=1.000000)" 0.0)
    (for _array_element (Variables|Don'tEdit|GetConditions)
      (Development|PrintString (Utilities|GetDisplayName _array_element) true true "(R=0.917376,G=1.000000,B=0.000000,A=1.000000)" 0.0))))

(event Input|KeyboardEvents|1
  (params (Key :type Key%20Structure :default "None"))
  ;[1 0.4074 0] DEBUG
  (:Pressed
    (CallFunction|AddShield 100)))

(event Input|KeyboardEvents|2
  (params (Key :type Key%20Structure :default "None"))
  ;[1 0.4074 0] DEBUG
  (:Pressed
    (CallFunction|RemoveHealth 320)))

(event Input|KeyboardEvents|3
  (params (Key :type Key%20Structure :default "None"))
  ;[1 0.4074 0] DEBUG
  (:Pressed
    (CallFunction|AddLevel 1)))

(event Input|KeyboardEvents|4
  (params (Key :type Key%20Structure :default "None"))
  ;[1 0.4074 0] DEBUG
  (:Pressed
    (CallFunction|AddHeal 60)))

(event Input|KeyboardEvents|5
  (params (Key :type Key%20Structure :default "None"))
  ;[1 0.4074 0] DEBUG
  (:Pressed
    (CallFunction|RemoveMana 100)))

(event Input|KeyboardEvents|6
  (params (Key :type Key%20Structure :default "None"))
  ;[1 0.4074 0] DEBUG
  (:Pressed
    (CallFunction|AddMana 50)))

(event Input|KeyboardEvents|7
  (params (Key :type Key%20Structure :default "None"))
  ;[1 0.4074 0] DEBUG
  (:Pressed
    (CallFunction|AddCondition "NewEnumerator1" 1e+01 (Game|Player|GetPlayerPawn 0))))

(event Input|KeyboardEvents|8
  (params (Key :type Key%20Structure :default "None"))
  ;[1 0.4074 0] DEBUG
  (:Pressed
    (CallFunction|AddCondition "NewEnumerator2" 1e+01 (Game|Player|GetPlayerPawn 0))))

(fn AddLevel
  (params (LevelsToAdd :type Integer))
  (if (CallFunction|IsAlive)
    (Variables|Don'tEdit|SetLevel (+ LevelsToAdd (Variables|Don'tEdit|GetLevel)))
    (if (.HealToFullOnLevelUp (Utilities|Struct|BreakS_HealthBar (Variables|!HealthBarSettings|GetSettings)))
      (CallFunction|AddHeal (Variables|Don'tEdit|GetMaxHealth)))
    (Default|CallOnLevelChange)))

(fn AddHeal
  (params (Value :type Integer))
  (bind _sounds (CallFunction|GetSounds))
  (bind _gettinghealsound (Utilities|Struct|BreakS_HealthBarSounds _sounds))
  (if (CallFunction|IsAlive)
    (Variables|Don'tEdit|SetCurrentHealth (Math|Integer|Clamp(Integer) (+ (Variables|Don'tEdit|GetCurrentHealth) Value) 0 (Variables|Don'tEdit|GetMaxHealth)))
    (Default|CallOnHealthChange)
    (Utilities|IsValid _gettinghealsound
      (:Is%20Valid
        (Audio|PlaySound2D _gettinghealsound 1.0 1.0 0.0 0 (Components|GetOwner) false)))))

(fn AddShield
  (params (Shield :type Integer))
  (bind _sounds (CallFunction|GetSounds))
  (bind _gettingshieldsound (Utilities|Struct|BreakS_HealthBarSounds _sounds))
  (if (CallFunction|IsAlive)
    (Variables|Don'tEdit|SetCurrentShield (+ (Variables|Don'tEdit|GetCurrentShield) Shield))
    (Default|CallOnHealthChange)
    (Utilities|IsValid _gettingshieldsound
      (:Is%20Valid
        (Audio|PlaySound2D _gettingshieldsound 1.0 1.0 0.0 0 (Components|GetOwner) false)))))

(fn AddMana
  (params (Value :type Integer))
  (bind _sounds (CallFunction|GetSounds))
  (bind _gettingmanasound (Utilities|Struct|BreakS_HealthBarSounds _sounds))
  (if (CallFunction|IsAlive)
    (Variables|Don'tEdit|SetCurrentMana (Math|Integer|Clamp(Integer) (+ (Variables|Don'tEdit|GetCurrentMana) Value) 0 (Variables|Don'tEdit|GetMaxMana)))
    (Default|CallOnManaChange)
    (Utilities|IsValid _gettingmanasound
      (:Is%20Valid
        (Audio|PlaySound2D _gettingmanasound 1.0 1.0 0.0 0 (Components|GetOwner) false)))))

(fn AddCondition
  (params (Condition :type EN_Conditions%20Enum :default "NewEnumerator1") (Duration%20%28seconds%29 :type Float%20%28double-precision%29) (Instigator :type Pawn%20Object%20Reference))
  (Utilities|IsValid Instigator
    (:Is%20Valid
      (LocalVariables|SetL%20Instigator Instigator))
    (:Is%20Not%20Valid
      (LocalVariables|SetL%20Instigator 0)))
  (LocalVariables|SetL%20Component%20Owner (Components|GetOwner))
  (switch Utilities|FlowControl|Switch|SwitchonEN_Conditions Condition
    (:NewEnumerator1
      (bind _returnvalue (Game|SpawnActorfromClass "/Game/SimpleHealthBar/Blueprints/Conditions/BP_PoisonCondition.BP_PoisonCondition_C" (Math|Transform|MakeTransform "0, 0, 0" "0, 0, 0" "1.000000,1.000000,1.000000") "AlwaysSpawn" "MultiplyWithRoot" (LocalVariables|GetL%20Component%20Owner) 10 Duration%20%28seconds%29 Instigator))
      (bind _condition (Utilities|AttachCondition _returnvalue)
        (:Success
          (Default|CallOnConditionAdded _condition))))
    (:NewEnumerator2
      (bind _returnvalue_2 (Game|SpawnActorfromClass "/Game/SimpleHealthBar/Blueprints/Conditions/BP_BurnCondition.BP_BurnCondition_C" (Math|Transform|MakeTransform "0, 0, 0" "0, 0, 0" "1.000000,1.000000,1.000000") "AlwaysSpawn" "MultiplyWithRoot" (LocalVariables|GetL%20Component%20Owner) 10 Duration%20%28seconds%29 Instigator))
      (bind _condition_2 (Utilities|AttachCondition _returnvalue_2)
        (:Success
          (Default|CallOnConditionAdded _condition_2))))))

(fn SetStartingLevel
  (if (<= (Variables|Don'tEdit|GetLevel) 0)
    (Variables|Don'tEdit|SetLevel 1))
  (return))

(fn SetLevel
  (params (Set%20Level%20To :type Integer))
  (Variables|Don'tEdit|SetLevel Set%20Level%20To)
  (Default|CallOnLevelChange))

(fn SetBaseHealthandManaValues
  (bind _settings (Variables|!HealthBarSettings|GetSettings))
  (bind (_healtofullonlevelup _unittype _basehealth _basemana) (Utilities|Struct|BreakS_HealthBar _settings))
  (Variables|Don'tEdit|SetMaxHealth _basehealth)
  (Variables|Don'tEdit|SetCurrentHealth _basehealth)
  (Variables|Don'tEdit|SetCurrentMana _basemana)
  (Variables|Don'tEdit|SetMaxMana _basemana))

(fn SetHealthandManaonLevelUp
  (bind _settings (Variables|!HealthBarSettings|GetSettings))
  (bind _settings_2 (Variables|!HealthBarSettings|GetSettings))
  (bind _level (Variables|Don'tEdit|GetLevel))
  (bind (_healtofullonlevelup _unittype _basehealth _basemana _healthperlevel _manaperlevel) (Utilities|Struct|BreakS_HealthBar _settings_2))
  (bind (_healthperlevel_2 _manaperlevel_2) (Utilities|Struct|BreakS_HealthBar _settings))
  (bind _returnvalue (- _level 1))
  (Variables|Don'tEdit|SetMaxHealth (+ _basehealth (* _returnvalue _healthperlevel)))
  (Variables|Don'tEdit|SetMaxMana (+ (* _returnvalue _manaperlevel) _basemana))
  (if _healtofullonlevelup
    (Variables|Don'tEdit|SetCurrentHealth (Variables|Don'tEdit|GetMaxHealth))
    (Variables|Don'tEdit|SetCurrentMana (Variables|Don'tEdit|GetMaxMana))
    (else
      (Variables|Don'tEdit|SetCurrentHealth (+ (Variables|Don'tEdit|GetCurrentHealth) _healthperlevel_2))
      (Variables|Don'tEdit|SetCurrentMana (+ (Variables|Don'tEdit|GetCurrentMana) _manaperlevel_2)))))

(fn RemoveHealth
  (params (Value :type Integer))
  (if (CallFunction|HasShield)
    (LocalVariables|SetL_RemainingDamage (- (Variables|Don'tEdit|GetCurrentShield) Value))
    (Variables|Don'tEdit|SetCurrentShield (Math|Integer|Clamp(Integer) (- (Variables|Don'tEdit|GetCurrentShield) Value) 0 (Variables|Don'tEdit|GetCurrentShield)))
    (if (< (LocalVariables|GetL_RemainingDamage) 0)
      (Variables|Don'tEdit|SetCurrentHealth (Math|Integer|Clamp(Integer) (- (Variables|Don'tEdit|GetCurrentHealth) (* (LocalVariables|GetL_RemainingDamage) -1)) 0 (Variables|Don'tEdit|GetMaxHealth)))
      (Default|CallOnHealthChange)
      (return)
      (else
        (Default|CallOnHealthChange)
        (return)))
    (else
      (Variables|Don'tEdit|SetCurrentHealth (Math|Integer|Clamp(Integer) (- (Variables|Don'tEdit|GetCurrentHealth) Value) 0 (Variables|Don'tEdit|GetMaxHealth)))
      (Default|CallOnHealthChange)
      (return))))

(fn RemoveMana
  (params (Value :type Integer))
  (Variables|Don'tEdit|SetCurrentMana (Math|Integer|Clamp(Integer) (- (Variables|Don'tEdit|GetCurrentMana) Value) 0 (Variables|Don'tEdit|GetMaxMana)))
  (Default|CallOnManaChange)
  (return))

(fn RemoveCondition
  (params (Condition :type Actor%20Object%20Reference))
  (Utilities|Array|RemoveItem (Variables|Don'tEdit|GetConditions) Condition)
  (Default|CallOnConditionRemoved))

(fn GetSounds
  (return (.Sounds (Utilities|Struct|BreakS_HealthBar (Variables|!HealthBarSettings|GetSettings)))))

(fn HasShield
  (return (> (Variables|Don'tEdit|GetCurrentShield) 0)))

(fn IsAlive
  (return (> (Variables|Don'tEdit|GetCurrentHealth) 0)))