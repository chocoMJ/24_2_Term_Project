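; Burn status condition actor that deals repeated fire damage to its owner, provided the owner has an AC_HealthBar component.
; On BeginPlay it starts a looping half-second damage timer and a one-shot timer for the condition's duration.
; Each tick applies BP_FireDamage, crediting the instigator when valid.
; On expiry it calls TimeoutCondition with the tick timer handle, removes itself from the health bar component and destroys itself.
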(event Custom|RunCondition
  (bind _returnvalue (Components|GetOwner))
  (bind _returnvalue_2 (Game|GetInstigator))
  ;[1 1 1] Your condition logic
  (Utilities|IsValid _returnvalue_2
    (:Is%20Valid
      (Game|Damage|ApplyDamage _returnvalue (Math|Conversions|ToFloat(Integer) (Variables|Default|GetFireTickDamage)) (Game|GetInstigatorController _returnvalue_2) _returnvalue_2 "/Game/SimpleHealthBar/Blueprints/DamageTypes/BP_FireDamage.BP_FireDamage_C"))
    (:Is%20Not%20Valid
      (Game|Damage|ApplyDamage _returnvalue (Math|Conversions|ToFloat(Integer) (Variables|Default|GetFireTickDamage)) 0 0 "/Game/SimpleHealthBar/Blueprints/DamageTypes/BP_FireDamage.BP_FireDamage_C"))))

(event Custom|RemoveCondition
  ;[1 1 1] Your condition logic
  (CallFunction|TimeoutCondition (Variables|Default|GetTimerHandle))
  (Default|RemoveCondition (Variables|Default|GetAC_HealthBar) self)
  (Actor|DestroyActor))

(event EventBeginPlay
  (bind _returnvalue (Components|GetOwner))
  (bind _returnvalue_2 (Actor|GetComponentbyClass _returnvalue "/Game/SimpleHealthBar/ActorComponents/AC_HealthBar.AC_HealthBar_C"))
  ;[1 1 1] Check if owner has AC_HealthBar component (it won't work otherwise)
  (Utilities|IsValid _returnvalue_2
    (:Is%20Valid
      (Variables|Default|SetAC_HealthBar _returnvalue_2)
      ;[1 1 1] Your condition logic
      (bind _returnvalue_3 (Utilities|Time|SetTimerbyEvent (delegate Custom|RunCondition) 0.5 true true))
      (Variables|Default|SetTimerHandle _returnvalue_3)
      (Utilities|Time|SetTimerbyEvent (delegate Custom|RemoveCondition) (Variables|Default|GetConditionTime) false true))))

(fn ConstructionScript
  (|CallParentFunction))