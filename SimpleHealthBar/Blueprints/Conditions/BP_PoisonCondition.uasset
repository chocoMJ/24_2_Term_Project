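; Poison condition actor for the health bar system that deals damage over time to its owner.
; On BeginPlay, if the owner has an AC_HealthBar, it starts a once-per-second damage tick and a one-shot expiry timer.
; Ticks apply BP_PoisonDamage, credited to the instigator when valid, through an event still named FearCondition.
; On expiry it times out the tick, removes itself from the health bar and destroys itself.
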(event Custom|FearCondition
  (bind _returnvalue (Game|GetInstigator))
  (Utilities|IsValid _returnvalue
    (:Is%20Valid
      (Game|Damage|ApplyDamage (Components|GetOwner) (Math|Conversions|ToFloat(Integer) (Variables|Default|GetPoisonTickDamage)) (Game|GetInstigatorController _returnvalue) _returnvalue "/Game/SimpleHealthBar/Blueprints/DamageTypes/BP_PoisonDamage.BP_PoisonDamage_C"))
    (:Is%20Not%20Valid
      (Game|Damage|ApplyDamage (Components|GetOwner) (Math|Conversions|ToFloat(Integer) (Variables|Default|GetPoisonTickDamage)) 0 0 "/Game/SimpleHealthBar/Blueprints/DamageTypes/BP_PoisonDamage.BP_PoisonDamage_C"))))

(event Custom|RemoveCondition
  (CallFunction|TimeoutCondition (Variables|Default|GetFearTimerHandle))
  (Default|RemoveCondition (Variables|Default|GetAC_HealthBar) self)
  (Actor|DestroyActor))

(event EventBeginPlay
  (bind _returnvalue (Components|GetOwner))
  (bind _returnvalue_2 (Actor|GetComponentbyClass _returnvalue "/Game/SimpleHealthBar/ActorComponents/AC_HealthBar.AC_HealthBar_C"))
  (Utilities|IsValid _returnvalue_2
    (:Is%20Valid
      (Variables|Default|SetAC_HealthBar _returnvalue_2)
      (bind _returnvalue_3 (Utilities|Time|SetTimerbyEvent (delegate Custom|FearCondition) 1.0 true true))
      (Variables|Default|SetFearTimerHandle _returnvalue_3)
      (Utilities|Time|SetTimerbyEvent (delegate Custom|RemoveCondition) (Variables|Default|GetConditionTime) false true))))

(fn ConstructionScript
  (|CallParentFunction))