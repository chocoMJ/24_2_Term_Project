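; Sci-fi double sliding door that opens for the BP-REALFINAL actor once its KillElite2 flag is set, and closes behind it.
; BeginPlay caches both panels' closed positions and computes open positions offset oppositely along world Y.
; Overlapping Detect plays the opening timeline and Detect_2 the closing one, each lerping both panels.
; IsOpen and IsClose are set when their timelines finish and never reset, blocking later replays.
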(event OnComponentBeginOverlap(detect)
  (params (OverlappedComponent :type Primitive%20Component%20Object%20Reference) (OtherActor :type Actor%20Object%20Reference) (OtherComp :type Primitive%20Component%20Object%20Reference) (OtherBodyIndex :type Integer) (bFromSweep :type Boolean) (SweepResult :type Hit%20Result%20Structure%20%28by%20ref%29))
  (bind _asbp_realfinal (Utilities|Casting|CastToBP-REALFINAL OtherActor))
  (if (and (Variables|/Game/ThirdPerson_twtwtw/Blueprints/BP-REALFINAL.BP-REALFINAL_C|Getkill_elite_2 _asbp_realfinal) (not (Variables|Default|Getis_open)))
    (bind _door_open (Timeline|타임라인 Play)
      (:Update
        (Transformation|SetWorldLocation (Variables|Default|GetSci-fi_Game_Door_Free_01_Right_Door) (Math|Vector|Lerp(Vector) (Variables|Default|GetOrigin_right) (Variables|Default|Gettrans_right) _door_open) false false)
        (Transformation|SetWorldLocation (Variables|Default|GetSci-fi_Game_Door_Free_01_Left_Door) (Math|Vector|Lerp(Vector) (Variables|Default|GetOrigin_left) (Variables|Default|Gettrans_left) _door_open) false false))
      (:Finished
        (Variables|Default|Setis_open true)))))

(event OnComponentBeginOverlap(detect_2)
  (params (OverlappedComponent :type Primitive%20Component%20Object%20Reference) (OtherActor :type Actor%20Object%20Reference) (OtherComp :type Primitive%20Component%20Object%20Reference) (OtherBodyIndex :type Integer) (bFromSweep :type Boolean) (SweepResult :type Hit%20Result%20Structure%20%28by%20ref%29))
  (Utilities|Casting|CastToBP-REALFINAL OtherActor)
  (if (not (Variables|Default|Getis_close))
    (bind _close_door (Timeline|타임라인_1 Play)
      (:Update
        (Transformation|SetWorldLocation (Variables|Default|GetSci-fi_Game_Door_Free_01_Right_Door) (Math|Vector|Lerp(Vector) (Variables|Default|Gettrans_right) (Variables|Default|GetOrigin_right) _close_door) false false)
        (Transformation|SetWorldLocation (Variables|Default|GetSci-fi_Game_Door_Free_01_Left_Door) (Math|Vector|Lerp(Vector) (Variables|Default|Gettrans_left) (Variables|Default|GetOrigin_left) _close_door) false false))
      (:Finished
        (Variables|Default|Setis_close true)))))

(event EventBeginPlay
  (Variables|Default|SetOrigin_left (Transformation|GetWorldLocation (Variables|Default|GetSci-fi_Game_Door_Free_01_Left_Door)))
  (Variables|Default|SetOrigin_right (Transformation|GetWorldLocation (Variables|Default|GetSci-fi_Game_Door_Free_01_Right_Door)))
  (Variables|Default|Settrans_left (+ (Variables|Default|GetOrigin_left) "0.000000,-700.000000,0.000000"))
  (Variables|Default|Settrans_right (+ (Variables|Default|GetOrigin_right) "0.000000,700.000000,0.000000")))

(fn ConstructionScript)